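; MyGameCharacter is a character Blueprint that handles basic player movement, look and jump input.
; Axis inputs add movement along the actor's forward and right vectors for walking and strafing.
; Turn and look axes add controller yaw and pitch scaled by a Sensitivity variable, and the Jump action calls Jump on press.
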(event Input|ActionEvents|InputActionJump
  (params (Key :type Key%20Structure))
  (:Pressed
    (Character|Jump)))

(event Input|AxisEvents|InputAxisForward_Backward
  (params (AxisValue :type Float%20%28single-precision%29))
  ;[1 1 1] Forward, back, left and right
  (Pawn|Input|AddMovementInput (Transformation|GetActorForwardVector) AxisValue false))

(event Input|AxisEvents|InputAxisStrafe_Left_Right
  (params (AxisValue :type Float%20%28single-precision%29))
  ;[1 1 1] Forward, back, left and right
  (Pawn|Input|AddMovementInput (Transformation|GetActorRightVector) AxisValue false))

(event Input|AxisEvents|InputAxisRotate_Left_Right
  (params (AxisValue :type Float%20%28single-precision%29))
  ;[1 1 1] Rotate left, right & look up and down
  (Pawn|Input|AddControllerYawInput (* AxisValue (Variables|MouseSettings|GetSensitivity))))

(event Input|AxisEvents|InputAxisLook_Up_Down
  (params (AxisValue :type Float%20%28single-precision%29))
  ;[1 1 1] Rotate left, right & look up and down
  (Pawn|Input|AddControllerPitchInput (* AxisValue (Variables|MouseSettings|GetSensitivity))))

(fn ConstructionScript)